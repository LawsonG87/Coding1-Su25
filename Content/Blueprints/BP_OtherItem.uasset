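; BP_OtherItem is a pickup potion item that BP_ThirdPersonCharacterCustom can carry, drop and use.
; Overlapping its PickupTrigger asks the character to pick it up, and Pickup attaches its root to the hand_r socket.
; Drop detaches it and enables physics and collision on the potion mesh so it falls.
; The primary action prints a mana gain, clears the held item and destroys itself; the secondary action only prints a message.
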(event `self.PickupTrigger.OnComponentBeginOverlap`
  (params (OverlappedComponent :type "PrimitiveComponent Object Reference") (OtherActor :type "Actor Object Reference") (OtherComp :type "PrimitiveComponent Object Reference") (OtherBodyIndex :type Integer) (bFromSweep :type Boolean) (SweepResult :type "HitResult Structure (by ref)"))
  (`KismetSystemLibrary.PrintString` "Other item has been touched.")
  (bind _asbp_third_person_character_custom (cast `/Game/Blueprints/BP_ThirdPersonCharacterCustom` OtherActor))
  (`/Game/Blueprints/BP_ThirdPersonCharacterCustom.TryToPickUp` _asbp_third_person_character_custom self))

(event `self.Pickup`
  (params (ParentMesh :type "SkeletalMeshComponent Object Reference"))
  (`SceneComponent.K2_AttachToComponent` (`self.DefaultSceneRoot`) ParentMesh "hand_r" "SnapToTarget" "KeepRelative" "KeepRelative" true))

(event `self.Drop`
  (`SceneComponent.K2_DetachFromComponent` (`self.DefaultSceneRoot`) "KeepRelative" "KeepRelative" "KeepRelative" true) ; Don't follow the hand anymore
  (`PrimitiveComponent.SetSimulatePhysics` (`self.Potion`) true) ; Use gravity to fall
  (`PrimitiveComponent.SetCollisionEnabled` (`self.Potion`) "QueryAndPhysics") ; collide with the ground please
)

(event `self.PrimaryAction`
  (params (ref_thirdPersonCharCustom :type "/Game/Blueprints/BP_ThirdPersonCharacterCustom Object Reference"))
  (`KismetSystemLibrary.PrintString` "+10 mana")
  (set `/Game/Blueprints/BP_ThirdPersonCharacterCustom.HeldItem` null ref_thirdPersonCharCustom)
  (`self.K2_DestroyActor`))

(event `/Game/Blueprints/BPI_Item.SecondaryAction`
  (`KismetSystemLibrary.PrintString` "Here's your secondary action." true true (struct :`R` 0.291667 :`G` 0.041245 :`B` 0.179269 :`A` 1.0)))

(fn `UserConstructionScript`)